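; EnemyTurret is an enemy turret that turns to face the player character when its PawnSensing component sees one.
; On sight it sets the whole actor's rotation with a look-at toward the BP_FPS_Character, then checks a SpawnProjectile flag.
; That check leads nowhere: the firing chain, which launches an impulse-driven FirstPersonProjectile with a Delay-based cooldown, is disconnected, so the turret never shoots.
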(event OnSeePawn(PawnSensing)
  (params (Pawn :type Pawn%20Object%20Reference))
  (bind _asbp_fps_character (Utilities|Casting|CastToBP_FPS_Character Pawn))
  (Utilities|FlowControl|Sequence
    (:then_0
      (Transformation|SetActorRotation (Math|Rotator|FindLookatRotation (Transformation|GetActorLocation) (Transformation|GetActorLocation _asbp_fps_character))))
    (:then_1
      (if (Variables|Default|GetSpawnProjectile)
        _))))

(fn ConstructionScript)