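; BP_WeaponProjectile is a weapon projectile that applies damage to what it overlaps.
; On actor overlap, it sends its Damage through AffectHealthMessage to IDamagable actors not tagged Friendly, then destroys itself.
; Overlapping an actor without that interface also destroys it, while Friendly damagable actors leave it intact and unharmed.
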(event Collision|EventActorBeginOverlap
  (params (OtherActor :type Actor%20Object%20Reference))
  (if (Utilities|DoesObjectImplementInterface OtherActor "/Game/Heagney/Blueprints/iDamagable.iDamagable_C")
    (if (not (Actor|ActorHasTag OtherActor "Friendly"))
      (Class|IDamagable|AffectHealth(Message) OtherActor (Variables|Default|GetDamage))
      (Actor|DestroyActor))
    (else
      (Actor|DestroyActor))))

(fn ConstructionScript
  (|CallParentFunction))