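; KeyDoors is a Blueprint holding three floating key pickups, each paired with its own door.
; Tick spins the keys and plays a timeline that offsets them along a movement vector.
; Each capsule's overlap, filtered by a "character" substring in the other actor's name, runs a timeline that pitches its door open.
; The matching key is only hidden, not destroyed, and nothing disables the capsule afterwards.
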(event OnComponentBeginOverlap(Capsule2)
  (params (OverlappedComponent :type Primitive%20Component%20Object%20Reference) (OtherActor :type Actor%20Object%20Reference) (OtherComp :type Primitive%20Component%20Object%20Reference) (OtherBodyIndex :type Integer) (bFromSweep :type Boolean) (SweepResult :type Hit%20Result%20Structure%20%28by%20ref%29))
  ;[1 1 1] Picking up keys op[en the doors and Destroy the keys
  (if (Utilities|String|Contains (Utilities|GetDisplayName OtherActor) "character")
    (Utilities|FlowControl|Sequence
      (:then_0
        (bind _newtrack_0 (Timeline|Timeline_2 Play)
          (:Update
            (Transformation|SetRelativeRotation (Variables|Default|GetDoor2) (Math|Rotator|MakeRotator 0.0 _newtrack_0 0.0) false false))))
      (:then_1
        (Rendering|SetVisibility (Variables|Default|GetKey2) false false)))))

(event OnComponentBeginOverlap(Capsule3)
  (params (OverlappedComponent :type Primitive%20Component%20Object%20Reference) (OtherActor :type Actor%20Object%20Reference) (OtherComp :type Primitive%20Component%20Object%20Reference) (OtherBodyIndex :type Integer) (bFromSweep :type Boolean) (SweepResult :type Hit%20Result%20Structure%20%28by%20ref%29))
  ;[1 1 1] Picking up keys op[en the doors and Destroy the keys
  (if (Utilities|String|Contains (Utilities|GetDisplayName OtherActor) "character")
    (Utilities|FlowControl|Sequence
      (:then_0
        (bind _newtrack_0 (Timeline|Timeline_3 Play)
          (:Update
            (Transformation|SetRelativeRotation (Variables|Default|GetDoor3) (Math|Rotator|MakeRotator 0.0 _newtrack_0 0.0) false false))))
      (:then_1
        (Rendering|SetVisibility (Variables|Default|GetKey3) false false)))))

(event OnComponentBeginOverlap(Capsule1)
  (params (OverlappedComponent :type Primitive%20Component%20Object%20Reference) (OtherActor :type Actor%20Object%20Reference) (OtherComp :type Primitive%20Component%20Object%20Reference) (OtherBodyIndex :type Integer) (bFromSweep :type Boolean) (SweepResult :type Hit%20Result%20Structure%20%28by%20ref%29))
  ;[1 1 1] Picking up keys op[en the doors and Destroy the keys
  (if (Utilities|String|Contains (Utilities|GetDisplayName OtherActor) "character")
    (Utilities|FlowControl|Sequence
      (:then_0
        (bind _newtrack_0 (Timeline|Timeline_1 Play)
          (:Update
            (Transformation|SetRelativeRotation (Variables|Default|GetDoor1) (Math|Rotator|MakeRotator 0.0 _newtrack_0 0.0) false false))))
      (:then_1
        (Rendering|SetVisibility (Variables|Default|GetKey1) false false)))))

(event EventTick
  (params (DeltaSeconds :type Float%20%28single-precision%29))
  ;[1 1 1] Spins Keys
  (Transformation|AddWorldRotation (Variables|Default|GetKey1) "0,1.000000, 0" false false)
  ;[1 1 1] Actor Up and Down, With Vector
  (bind _movement (Timeline|Timeline_0 Play)
    (:Update
      (Transformation|AddWorldOffset (Variables|Default|GetKey1) _movement false false))))

(fn ConstructionScript)